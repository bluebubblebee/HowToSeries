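; BP_SashimiItemInteractive is an interactive, collectible sashimi item that disappears when picked up.
; On interact, if it is not already collected, it calls the parent's interact logic and plays a beep at its location.
; It then hides the Item component and disables collision on both Item and Trigger, leaving the actor in the world rather than destroying it.
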(event EventOnInteract
  (if (not (Variables|Default|GetbItemCollected))
    (|CallParentFunction)
    (Audio|PlaySoundatLocation "/UINavigation/Audio/Beep_1.Beep_1" (Transformation|GetActorLocation) "0, 0, 0" 1.0 1.0 0.0 0 0 0)
    (Rendering|SetVisibility (Variables|Default|GetItem) false false)
    (Collision|SetCollisionEnabled (Variables|Default|GetItem) "NoCollision")
    (Collision|SetCollisionEnabled (Variables|Default|GetTrigger) "NoCollision")))

(fn ConstructionScript)