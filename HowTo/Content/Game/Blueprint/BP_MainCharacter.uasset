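; Main character Blueprint that owns and drives the player's HUD for prompts, quests and inventory.
; BeginPlay creates the in-game, quest and inventory widgets and adds them to the viewport.
; Events forward prompt text, quest and completion messages to the in-game widget, and quest lists to the quest widget.
; Inventory refresh shows the inventory widget and fills it from EquipmentInventory; OnHideUI is left empty.
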(event EventOnHideUI)

(event EventOnShowQuestInfo
  (params (Quest :type Quest%20Structure))
  ;[1 0.4784 0.5765] Show Quest Info
  (Default|OnUpdateDialogueText (Variables|Default|GetInGameUI) (.message Quest)))

(event EventOnShowQuestCompleted
  (params (Message :type Text%20%28by%20ref%29))
  ;[1 0.4784 0.5765] Show Quest completed
  (Default|OnUpdateDialogueText (Variables|Default|GetInGameUI) Message))

(event EventOnShowUI
  (params (Character :type Name :default "None"))
  (Default|OnUpdatePromptText (Variables|Default|GetInGameUI) (Utilities|Text|ToText(Name) Character)))

(event EventOnShowUpdatedQuestList
  (params (QuestTextList :type Array%20of%20Texts))
  (bind _questui (Variables|Default|GetQuestUI))
  ;[1 0.4784 0.5765] Quest
  (if (Utilities|IsValid _questui)
    (Default|UpdateQuestList _questui QuestTextList)))

(event EventBeginPlay
  ;[1 0.4784 0.5765] Initialization
  (Utilities|FlowControl|Sequence
    (:then_0
      (bind _returnvalue (UserInterface|CreateWidget "/Game/Game/UI/WBP_InGameUI.WBP_InGameUI_C"))
      (UserInterface|Viewport|AddtoViewport _returnvalue 0)
      (Variables|Default|SetInGameUI _returnvalue))
    (:then_1
      (bind _returnvalue_2 (UserInterface|CreateWidget "/Game/Game/UI/Quest/WBP_Quest.WBP_Quest_C"))
      (UserInterface|Viewport|AddtoViewport _returnvalue_2 0)
      (Variables|Default|SetQuestUI _returnvalue_2))
    (:then_2
      (bind _returnvalue_3 (UserInterface|CreateWidget "/Game/Game/UI/Inventory/WBP_Inventory.WBP_Inventory_C"))
      (bind _output_get (Variables|Default|SetInventoryUI _returnvalue_3))
      (UserInterface|Viewport|AddtoViewport _output_get 0))))

(event EventOnRefreshInventory
  (bind _inventoryui (Variables|Default|GetInventoryUI))
  ;[1 0.4784 0.5765] OnRefreshInventory
  (if (Utilities|IsValid _inventoryui)
    (Default|Show _inventoryui)
    (Default|RefreshInventory _inventoryui (Variables|Default|GetEquipmentInventory))))

(fn ConstructionScript)