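; BP_FloatingRobot is a small robot actor that shows a selectable face on its skeletal mesh.
; On BeginPlay it creates a dynamic instance of the mesh's second material slot, then waits briefly before applying the selection.
; The clamped column sets the UV U offset in quarter steps.
; The clamped row picks the V offset: row zero sets it directly, while each other row plays its own timeline to drive it.
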(event EventBeginPlay
  (bind _skeletalmesh (Variables|Default|GetSkeletalMesh))
  (bind _returnvalue (Rendering|Material|CreateDynamicMaterialInstance _skeletalmesh 1 (Rendering|Material|GetMaterial _skeletalmesh 1) "None" :!class /Script/Engine.PrimitiveComponent))
  (bind _output_get (Variables|Default|SetMI_Face _returnvalue))
  (Rendering|Material|SetMaterial (Variables|Default|GetSkeletalMesh) 1 _output_get)
  (Utilities|FlowControl|Delay 2.0)
  (Rendering|Material|SetScalarParameterValue (Variables|Default|GetMI_Face) "UOffset" (* (Math|Integer|Clamp(Integer) (Variables|Default|GetSelectedColumn) 0 (Variables|Default|GetMaxColumn)) 0.25) :!class /Script/Engine.MaterialInstanceDynamic)
  (switch int (Math|Integer|Clamp(Integer) (Variables|Default|GetSelectedRow) 0 (Variables|Default|GetMaxRow))
    (:0
      (Rendering|Material|SetScalarParameterValue (Variables|Default|GetMI_Face) "VOffset" 0.0 :!class /Script/Engine.MaterialInstanceDynamic))
    (:1
      (bind _offset (Timeline|Row1 Play)
        (:Update
          (Rendering|Material|SetScalarParameterValue (Variables|Default|GetMI_Face) "VOffset" _offset :!class /Script/Engine.MaterialInstanceDynamic))))
    (:2
      (bind _offset_2 (Timeline|Row2 Play)
        (:Update
          (Rendering|Material|SetScalarParameterValue (Variables|Default|GetMI_Face) "VOffset" _offset_2 :!class /Script/Engine.MaterialInstanceDynamic))))
    (:3
      (bind _offset_3 (Timeline|Timeline Play)
        (:Update
          (Rendering|Material|SetScalarParameterValue (Variables|Default|GetMI_Face) "VOffset" _offset_3 :!class /Script/Engine.MaterialInstanceDynamic))))))

(fn ConstructionScript)